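; Healing spell from the UI kit showcase that restores health to the caster's Example_Character when cast.
; CastFunction casts the user's controlled pawn, then adds HealAmount to current health, capped at maximum.
; It then updates the "health" bar, but recomputes the percentage from the already-healed value, so HealAmount counts twice in the display until the cap.
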(event EventCastFunction
  (params (User :type Player%20Controller%20Object%20Reference))
  (bind _asexample_character (Utilities|Casting|CastToExample_Character (Pawn|GetControlledPawn User)))
  (Variables|/Game/UI_Kit/Showcase/Blueprints/Example_Character.Example_Character_C|SetCurrent%20Health _asexample_character (Math|Float|Min(Float) (+ (Variables|/Game/UI_Kit/Showcase/Blueprints/Example_Character.Example_Character_C|GetCurrent%20Health _asexample_character) (Variables|Default|GetHeal%20Amount)) (Variables|/Game/UI_Kit/Showcase/Blueprints/Example_Character.Example_Character_C|GetMaximum%20Health _asexample_character)))
  (Default|CallUpdateABar _asexample_character "health" (/ (Math|Float|Min(Float) (+ (Variables|/Game/UI_Kit/Showcase/Blueprints/Example_Character.Example_Character_C|GetCurrent%20Health _asexample_character) (Variables|Default|GetHeal%20Amount)) (Variables|/Game/UI_Kit/Showcase/Blueprints/Example_Character.Example_Character_C|GetMaximum%20Health _asexample_character)) (Variables|/Game/UI_Kit/Showcase/Blueprints/Example_Character.Example_Character_C|GetMaximum%20Health _asexample_character))))

(event EventBeginPlay)

(event EventActorBeginOverlap
  (params (OtherActor :type Actor%20Object%20Reference)))

(event EventTick
  (params (DeltaSeconds :type Float%20%28single-precision%29)))

(fn ConstructionScript
  (|CallParentFunction))