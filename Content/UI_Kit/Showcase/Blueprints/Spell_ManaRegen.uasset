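; Showcase spell Blueprint that grants a temporary mana regeneration boost to the casting user's Example_Character pawn.
; CastFunction adds ExtraManaRegen to the character's ManaRegenPerSec, then subtracts it after a delay of Seconds.
; A Gate closes for the duration of the boost and reopens afterward, so repeat casts on the same spell instance do not stack.
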(event EventBeginPlay)

(event EventActorBeginOverlap
  (params (OtherActor :type Actor%20Object%20Reference)))

(event EventTick
  (params (DeltaSeconds :type Float%20%28single-precision%29)))

(event EventCastFunction
  (params (User :type Player%20Controller%20Object%20Reference))
  (bind _asexample_character (Utilities|Casting|CastToExample_Character (Pawn|GetControlledPawn User)))
  (Utilities|FlowControl|Gate false :!label _label
    (:Exit
      (Variables|/Game/UI_Kit/Showcase/Blueprints/Example_Character.Example_Character_C|SetMana%20Regen%20Per%20Sec _asexample_character (+ (Variables|/Game/UI_Kit/Showcase/Blueprints/Example_Character.Example_Character_C|GetMana%20Regen%20Per%20Sec _asexample_character) (Variables|Default|GetExtra%20Mana%20Regen)))
      (Utilities|FlowControl|Sequence
        (:then_0
          (goto _label Close))
        (:then_1
          (Utilities|FlowControl|Delay (Variables|Default|GetSeconds))
          (Variables|/Game/UI_Kit/Showcase/Blueprints/Example_Character.Example_Character_C|SetMana%20Regen%20Per%20Sec _asexample_character (- (Variables|/Game/UI_Kit/Showcase/Blueprints/Example_Character.Example_Character_C|GetMana%20Regen%20Per%20Sec _asexample_character) (Variables|Default|GetExtra%20Mana%20Regen)))
          (goto _label Open))))))

(fn ConstructionScript
  (|CallParentFunction))